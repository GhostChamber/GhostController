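; BP_RotatingModel is an actor that rotates and scales itself and reports its transform over the network.
; Setter functions control rotation speed, per-axis direction and scale factor.
; Tick applies delta-time-scaled rotation while direction is non-zero, and multiplies scale every frame while the factor is non-zero.
; After either change, it sends rotation and X scale as a string through GhostNetworkClient, which starts discovery on BeginPlay.
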(fn `GetMessageString`
  (returns (OutputString :type String))
  (return (`KismetTextLibrary.Conv_TextToString` (`|FormatText` "{Pitch} {Yaw} {Roll} {Scale}" (.pitch (`self.K2_GetActorRotation`)) (.yaw (`self.K2_GetActorRotation`)) (.roll (`self.K2_GetActorRotation`)) (.x (`self.GetActorScale3D`))))))

(fn `Rotate`
  ;[0.1674 0.5601 1] Rotate
  (`self.K2_SetActorRotation` (`KismetMathLibrary.ComposeRotators` (`KismetMathLibrary.MakeRotator` (.x (* (`self.RotationDirection`) (* (`self.DeltaSeconds`) (`self.RotationSpeed`)))) (.y (* (`self.RotationDirection`) (* (`self.DeltaSeconds`) (`self.RotationSpeed`)))) (.z (* (`self.RotationDirection`) (* (`self.DeltaSeconds`) (`self.RotationSpeed`))))) (`self.K2_GetActorRotation`))))

(fn `Scale`
  (`self.SetActorScale3D` (* (`self.GetActorScale3D`) (`self.ScaleFactor`))))

(fn `SetPitchDirection`
  (params (PitchDir :type Integer))
  (set `self.RotationDirection` (`KismetMathLibrary.MakeVector` (.x (`self.RotationDirection`)) (`KismetMathLibrary.Conv_IntToDouble` PitchDir) (.z (`self.RotationDirection`)))))

(fn `SetRollDirection`
  (params (RollDir :type Integer))
  (set `self.RotationDirection` (`KismetMathLibrary.MakeVector` (`KismetMathLibrary.Conv_IntToDouble` RollDir) (.y (`self.RotationDirection`)) (.z (`self.RotationDirection`)))))

(fn `SetRotationSpeed`
  (params (Speed :type "Float (double-precision)"))
  (set `self.RotationSpeed` Speed))

(fn `SetScaleFactor`
  (params (ScaleFactor :type "Float (double-precision)"))
  (set `self.ScaleFactor` ScaleFactor))

(fn `SetYawDirection`
  (params (YawDir :type Integer))
  (set `self.RotationDirection` (`KismetMathLibrary.MakeVector` (.x (`self.RotationDirection`)) (.y (`self.RotationDirection`)) (`KismetMathLibrary.Conv_IntToDouble` YawDir))))

(fn `UserConstructionScript`)